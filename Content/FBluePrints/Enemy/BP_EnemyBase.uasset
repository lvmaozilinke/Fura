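; BP_EnemyBase is a base enemy Blueprint that adds presentation behavior on top of its parent class.
; UpdateFacingTarget feeds a location to Motion Warping as the "FacingTarget" warp target.
; Two dissolve events play timelines that drive the "Dissolve" parameter on dynamic materials for the mesh and weapon.
; Tick draws a debug sphere while HightLightActor is set, and a leftover AttributeSet lookup is never executed.
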(event EventBeginPlay
  (|CallParentFunction))

(event Collision|EventActorBeginOverlap
  (params (OtherActor :type Actor%20Object%20Reference)))

(event EventTick
  (params (DeltaSeconds :type Float%20%28single-precision%29))
  (|CallParentFunction DeltaSeconds)
  (if (Variables|Default|GetbHightLightActor)
    (Rendering|Debug|DrawDebugSphere (Transformation|GetActorLocation) 1e+02 12 "(R=1.000000,G=1.000000,B=1.000000,A=1.000000)" 1.0 2.0)))

(event EventUpdateFacingTarget
  (params (TargetLocation :type Vector%20%28by%20ref%29 :default "0, 0, 0"))
  (Class|MotionWarpingComponent|AddorUpdateWarpTargetfromLocation (Variables|Default|GetMotionWarping) "FacingTarget" TargetLocation))

(event EventStartMeshDissolveTimeline
  (params (DynamicMaterialInstance :type Material%20Instance%20Dynamic%20Object%20Reference))
  ;[1 1 1] 溶解
  (bind _track (Timeline|时间轴 PlayFromStart)
    (:Update
      (Rendering|Material|SetScalarParameterValue DynamicMaterialInstance "Dissolve" _track :!class /Script/Engine.MaterialInstanceDynamic))))

(event EventStartWeaponDissolveTimeline
  (params (DynamicMaterialInstance :type Material%20Instance%20Dynamic%20Object%20Reference))
  ;[1 1 1] 溶解
  (bind _track (Timeline|时间轴_0 PlayFromStart)
    (:Update
      (Rendering|Material|SetScalarParameterValue DynamicMaterialInstance "Dissolve" _track :!class /Script/Engine.MaterialInstanceDynamic))))

(fn ConstructionScript)