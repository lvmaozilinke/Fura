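; Melee attack gameplay ability that plays the goblin spear attack montage on its avatar.
; On activation it turns the avatar toward its combat target through the combat interface, then waits for the melee montage gameplay event.
; The event triggers a radius search for live players around the combat socket, excluding the avatar.
; Hits are only drawn as debug spheres, with no damage applied, before the ability ends.
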(event Ability|EventActivateAbility
  (bind _returnvalue (Ability|GetAvatarActorfromActorInfo))
  (bind _returnvalue_2 (Ability|GetAvatarActorfromActorInfo))
  (bind _returnvalue_3 (Class|EnemyInterfaceF|GetCombatTarget(Message) _returnvalue_2))
  (Development|PrintString (Utilities|GetObjectName _returnvalue_3))
  (bind _ascombat_interface_f (Utilities|Casting|CastToCombatInterface_F _returnvalue_2))
  ;[1 1 1] 看向目标处
  (Class|CombatInterfaceF|UpdateFacingTarget _ascombat_interface_f (Transformation|GetActorLocation _returnvalue_3))
  (|PlayMontageandWaitProxy "None" "/Game/Assets/Enemies/Goblin/Animations/Spear/AM_Attack_GoblinSpear_F.AM_Attack_GoblinSpear_F" 1.0 "None" true 1.0 0.0 false
    (:then
      (Ability|Tasks|WaitGameplayEvent "(TagName=\"FEvent.Montage.Attack.Melee\")" 0
        (:EventReceived
          (bind _returnvalue_4 (Class|CombatInterfaceF|GetCombatSocketLocation(Message) _returnvalue))
          (bind _outoverlappingactors (Class|FuraAbilitySystemLibrary|GetLivePlayersWithinRadius _returnvalue (Utilities|Array|MakeArray _returnvalue) 45.0 _returnvalue_4))
          (for _array_element _outoverlappingactors
            (Rendering|Debug|DrawDebugSphere (Transformation|GetActorLocation _array_element) 15.0 12 "(R=0.000000,G=0.235196,B=1.000000,A=1.000000)" 5.0))
          (Ability|EndAbility))))))