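; Enemy ranged attack gameplay ability that fires a projectile at the avatar's current combat target.
; On activation it turns the avatar toward the target through interface messages and plays a random tagged attack montage.
; A gameplay event matching that montage's tag triggers SpawnProjectile, using the target's location re-read at that moment.
; The graph also prints the target's name for debugging and contains no EndAbility call.
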(event Ability|EventActivateAbility
  (bind _returnvalue (Ability|GetAvatarActorfromActorInfo))
  (bind _returnvalue_2 (Ability|GetAvatarActorfromActorInfo))
  (bind _returnvalue_3 (Class|EnemyInterfaceF|GetCombatTarget(Message) _returnvalue))
  (Development|PrintString (Utilities|String|Append "GA_RangedAttack:" (Utilities|GetObjectName _returnvalue_3)))
  (Class|CombatInterfaceF|UpdateFacingTarget(Message) _returnvalue (Transformation|GetActorLocation _returnvalue_3))
  (bind _returnvalue_4 (Class|CombatInterfaceF|GetAttackMontages(Message) (Ability|GetAvatarActorfromActorInfo)))
  (bind _output_get (Variables|Default|SetToggedMontage (Class|FuraDamageGameplayAbility|GetRandomTaggedMontagefromArray _returnvalue_4)))
  (|PlayMontageandWaitProxy "None" (.Montage (Utilities|Struct|BreakTaggedMontage_F _output_get)) 1.0 "None" true 1.0 0.0 false
    (:then
      (Ability|Tasks|WaitGameplayEvent (.MontageTag (Utilities|Struct|BreakTaggedMontage_F _output_get)) 0
        (:EventReceived
          (Class|CombatInterfaceF|GetCombatSocketLocation(Message) _returnvalue_2 (.MontageTag (Utilities|Struct|BreakTaggedMontage_F _output_get)))
          (bind _returnvalue_5 (Class|EnemyInterfaceF|GetCombatTarget(Message) _returnvalue_2))
          (Class|FuraProjectileSpell|SpawnProjectile (Transformation|GetActorLocation _returnvalue_5)))))))