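; Enemy melee attack gameplay ability that turns the avatar toward its combat target and plays a randomly chosen tagged attack montage.
; When the montage's gameplay event fires, it finds live players in a small sphere at the tagged combat socket and damages non-friends, triggering their blood effect.
; A hit executes a melee impact GameplayCue carrying the montage tag to distinguish effects.
; The ability ends after the event is handled or the montage completes, is interrupted or cancelled.
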(event Ability|EventActivateAbility
  (bind _returnvalue (Ability|GetAvatarActorfromActorInfo))
  (bind _returnvalue_2 (Ability|GetAvatarActorfromActorInfo))
  (bind _returnvalue_3 (Ability|GetAvatarActorfromActorInfo))
  (Variables|Default|SetHasHitTarget false)
  (bind _returnvalue_4 (Class|EnemyInterfaceF|GetCombatTarget(Message) _returnvalue_2))
  (Development|PrintString (Utilities|String|Append "GA_MeleeAttack:" (Utilities|GetObjectName _returnvalue_4)))
  (bind _ascombat_interface_f (Utilities|Casting|CastToCombatInterface_F _returnvalue_2))
  ;[1 1 1] 看向目标处
  (Class|CombatInterfaceF|UpdateFacingTarget _ascombat_interface_f (Transformation|GetActorLocation _returnvalue_4))
  (bind _returnvalue_5 (Class|CombatInterfaceF|GetAttackMontages(Message) (Ability|GetAvatarActorfromActorInfo)))
  (Variables|Default|SetToggedMontage (Class|FuraDamageGameplayAbility|GetRandomTaggedMontagefromArray _returnvalue_5))
  (|PlayMontageandWaitProxy "None" (.Montage (Utilities|Struct|BreakTaggedMontage_F (Variables|Default|GetToggedMontage))) 1.0 "None" false 1.0 0.0 false
    (:then
      (Ability|Tasks|WaitGameplayEvent (.MontageTag (Utilities|Struct|BreakTaggedMontage_F (Variables|Default|GetToggedMontage))) 0 ; 蒙太奇动画标签触发
        (:EventReceived
          (bind _returnvalue_6 (Class|CombatInterfaceF|GetCombatSocketLocation(Message) _returnvalue_3 (.SocketTag (Utilities|Struct|BreakTaggedMontage_F (Variables|Default|GetToggedMontage)))))
          (Variables|Default|SetCombatSocketLocation _returnvalue_6)
          (bind _outoverlappingactors (Class|FuraAbilitySystemLibrary|GetLivePlayersWithinRadius _returnvalue_3 (Utilities|Array|MakeArray _returnvalue_3) 45.0 (Variables|Default|GetCombatSocketLocation)))
          (for _array_element _outoverlappingactors
            (if (Class|FuraAbilitySystemLibrary|IsNotFriend (Ability|GetAvatarActorfromActorInfo) _array_element) ; 是否不是友方
              (Class|FuraDamageGameplayAbility|CauseDamage _array_element)
              (Variables|Default|SetHasHitTarget true) ; 找到伤害目标,标记命中，然后播放音频音效
              ;[1 1 1] 播放命中特效
              (Class|CombatInterfaceF|GetBloodEffect(Message) _array_element)))
          (if (Variables|Default|GetHasHitTarget)
            (bind _returnvalue_7 (Class|EnemyInterfaceF|GetCombatTarget(Message) _returnvalue))
            ;[1 1 1] 命中播放音效-调用gameplaycue
            (Class|GameplayAbility|ExecuteGameplayCuewithParams "(TagName=\"GameplayCue.MeleeImpact_F\")" (Ability|GameplayCue|MakeGameplayCueParameters :AggregatedSourceTags (GameplayTags|MakeGameplayTagContainerfromTag (.MontageTag (Utilities|Struct|BreakTaggedMontage_F (Variables|Default|GetToggedMontage)))) :Location (Variables|Default|GetCombatSocketLocation) :EffectCauser _returnvalue :SourceObject _returnvalue_7)))
          (Ability|EndAbility))))
    (:OnCompleted
      (Ability|EndAbility :!label _label))
    (:OnInterrupted
      (goto _label))
    (:OnCancelled
      (goto _label))))