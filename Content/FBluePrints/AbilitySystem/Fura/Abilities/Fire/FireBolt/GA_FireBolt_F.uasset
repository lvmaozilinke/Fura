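; GA_FireBolt_F is a gameplay ability that casts a fire bolt projectile toward the point under the mouse.
; It waits for cursor target data, turns the avatar to face that location through the combat interface, and plays the cast montage.
; A montage gameplay event triggers spawning the projectile from the weapon socket toward the target.
; The ability ends when the montage completes, blends out, is interrupted or cancelled.
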(event Ability|EventActivateAbility
  (bind _datahandle (|TargetDataUnderMouseF)
    (:ValidData
      (Variables|Default|SetProjectileTargetLocation (.Location (Collision|BreakHitResult (Ability|TargetData|GetHitResultfromTargetData _datahandle))))
      (bind _ascombat_interface_f (Utilities|Casting|CastToCombatInterface_F (Ability|GetAvatarActorfromActorInfo)))
      (Class|CombatInterfaceF|UpdateFacingTarget _ascombat_interface_f (Variables|Default|GetProjectileTargetLocation))
      (|PlayMontageandWaitProxy "None" "/Game/Assets/Characters/Aura/Animations/Abilities_F/AM_Cast_FireBolt_F.AM_Cast_FireBolt_F" 1.0 "None" true 1.0 0.0 false
        (:then
          ;[1 1 1] 注释
          (Ability|Tasks|WaitGameplayEvent "(TagName=\"FEvent.Montage.FireBolt\")" 0
            (:EventReceived
              (Development|PrintString "EM.FireBolt Is Received") ; 已收到
              (Class|FuraProjectileSpell|SpawnProjectile (Variables|Default|GetProjectileTargetLocation) (GameplayTags|MakeLiteralGameplayTag "(TagName=\"FCombatSocket.Weapon\")")))))
        (:OnCompleted
          ;[1 1 1] 很重要，必须执行此节点结束能力，不然不会执行下一个能力
          (Ability|EndAbility :!label _label))
        (:OnBlendOut
          (goto _label))
        (:OnInterrupted
          (goto _label))
        (:OnCancelled
          (goto _label))))))

(event Ability|EventOnEndAbility
  (params (bWasCancelled :type Boolean)))